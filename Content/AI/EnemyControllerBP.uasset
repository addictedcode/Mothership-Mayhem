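; Enemy AI controller that maintains the PlayerFeet blackboard key from the current target's Floor.
; On possession and on ChangeTarget, it reads the Target key and, if that is a BP_MMCharacterBase, stores its Floor.
; Otherwise it casts the NewTarget event argument, rather than the blackboard Target, to DefensePod and stores that Floor instead.
; ChangeTarget never writes the Target key itself.
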(event `self.ReceivePossess`
  (params (PossessedPawn :type "Pawn Object Reference"))
  (bind _playerfeet (`self.PlayerFeet`))
  (bind _returnvalue (`AIBlueprintHelperLibrary.GetBlackboard` self))
  (`parent.ReceivePossess` PossessedPawn)
  (bind _asbp_mmcharacter_base (cast `/Game/Blueprints/Characters/BP_MMCharacterBase` (`BlackboardComponent.GetValueAsObject` _returnvalue (`self.Target`)) :!label _label)
    (:`then`
      (`BlackboardComponent.SetValueAsObject` _returnvalue _playerfeet (`/Game/Blueprints/Characters/BP_MMCharacterBase.Floor` _asbp_mmcharacter_base)))
    (:`CastFailed`
      (bind _asdefense_pod (cast `/Game/Blueprints/Interactables/DefensePod` (stale `self.ChangeTarget` newTarget)))
      (`BlackboardComponent.SetValueAsObject` _returnvalue _playerfeet (`/Game/Blueprints/Interactables/DefensePod.Floor` _asdefense_pod)))))

(event `self.ChangeTarget`
  (params (newTarget :type "Actor Object Reference"))
  (goto _label))

(event `self.ReceiveBeginPlay`)

(event `self.ReceiveTick`
  (params (DeltaSeconds :type "Float (single-precision)")))

(fn `UserConstructionScript`)