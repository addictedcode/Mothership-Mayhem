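; BP_Boss1Slam is an expanding slam shockwave for Boss 1 that damages and knocks up characters it touches.
; Activate moves it to a start location and enables expansion, then Tick grows its X and Y scale until ExpansionLimit, where it destroys itself.
; Cylinder overlaps deal fixed damage to BP_MMCharacterBase actors and teleport them upward by KnockupHeight instead of launching them.
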(event `self.ReceiveTick`
  (params (DeltaSeconds :type "Float (single-precision)"))
  (bind _returnvalue (* 20 DeltaSeconds))
  (bind _returnvalue_2 (`KismetMathLibrary.MakeVector` (+ (.x (`self.GetActorScale3D`)) _returnvalue) (+ (.y (`self.GetActorScale3D`)) _returnvalue) (.z (`self.GetActorScale3D`))))
  (if (`self.isExpanding`)
    (`self.SetActorScale3D` _returnvalue_2)
    (if (>= (.x _returnvalue_2) (`self.ExpansionLimit`))
      (set `self.isExpanding` false)
      (`self.K2_DestroyActor`))))

(event `self.Cylinder.OnComponentBeginOverlap`
  (params (OverlappedComponent :type "PrimitiveComponent Object Reference") (OtherActor :type "Actor Object Reference") (OtherComp :type "PrimitiveComponent Object Reference") (OtherBodyIndex :type Integer) (bFromSweep :type Boolean) (SweepResult :type "HitResult Structure (by ref)"))
  (bind _asbp_mmcharacter_base (cast `/Game/Blueprints/Characters/BP_MMCharacterBase` OtherActor))
  (`/Game/Blueprints/Characters/BP_MMCharacterBase.TakeDamage` _asbp_mmcharacter_base 70)
  (`self.K2_SetActorLocation` _asbp_mmcharacter_base (+ (`self.K2_GetActorLocation` _asbp_mmcharacter_base) (`KismetMathLibrary.MakeVector` 0.0 0.0 (`self.Knockup height`))) false true))

(fn `Activate`
  (params (StartLocation :type "Vector Structure"))
  (`self.K2_SetActorLocation` StartLocation false true)
  (set `self.isExpanding` true))

(fn `UserConstructionScript`)