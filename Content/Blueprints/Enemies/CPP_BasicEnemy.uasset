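; Basic enemy Blueprint that handles death rewards and damage number feedback.
; On DeathGang it spawns a random handful of battery drops in Defense game mode, then notifies the arena game mode of the kill.
; Capsule hits and overlaps from non-enemy projectiles show a DamagePopUP widget at the impact's screen position, without applying damage here.
; Tick is empty, with face-the-player rotation logic left disconnected.
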(event `self.DeathGang`
  ;[1 1 1] On Death Event
  (`|ExecutionSequence`
    (:`then_0`
      (cast `/Game/Blueprints/Gamemodes/MM_ArenaGameMode_Defense` (`GameplayStatics.GetGameMode`))
      ;;[1 1 1] Money Drop
      (for _ (range (+ (`KismetMathLibrary.RandomIntegerInRange` 1 5) 1))
        (`|SpawnActorFromClass` "/Game/Blueprints/Drops/Defense_BatteryDrop.Defense_BatteryDrop_C" (`KismetMathLibrary.Conv_VectorToTransform` (`self.K2_GetActorLocation` self)) "AdjustIfPossibleButAlwaysSpawn" "OverrideRootScale" null null)))
    (:`then_1`
      ;;[1 1 1] Enemy Count Decrement
      (bind _asmm_arena_game_mode (cast `/Game/Blueprints/Gamemodes/MM_ArenaGameMode` (`GameplayStatics.GetGameMode`)))
      (`/Game/Blueprints/Gamemodes/MM_ArenaGameMode.EnemyKilled` _asmm_arena_game_mode))))

(event `self.ReceiveTick`
  (params (DeltaSeconds :type "Float (single-precision)")))

(event `self.CapsuleComponent.OnComponentHit`
  (params (HitComponent :type "PrimitiveComponent Object Reference") (OtherActor :type "Actor Object Reference") (OtherComp :type "PrimitiveComponent Object Reference") (NormalImpulse :type "Vector Structure") (Hit :type "HitResult Structure (by ref)"))
  ;[1 1 1] On Hit
  (bind _asmmprojectile_base (cast `MMProjectileBase` OtherActor))
  (if (`|EnumInequality` (`MMProjectileBase.faction` _asmmprojectile_base) "Enemy")
    (bind _returnvalue (`|CreateWidget` "/Game/Blueprints/UI/ArenaChallengeUI/DamagePopUP.DamagePopUP_C"))
    (`UserWidget.AddToViewport` _returnvalue 0)
    (`/Game/Blueprints/UI/ArenaChallengeUI/DamagePopUP.Damage Text Pop Up Event` _returnvalue (`KismetMathLibrary.Round` (`MMProjectileBase.damage` _asmmprojectile_base)) (`GameplayStatics.ProjectWorldToScreen` (`GameplayStatics.GetPlayerController` 0) (`.Location` (`GameplayStatics.BreakHitResult` Hit)) true))))

(event `self.CapsuleComponent.OnComponentBeginOverlap`
  (params (OverlappedComponent :type "PrimitiveComponent Object Reference") (OtherActor :type "Actor Object Reference") (OtherComp :type "PrimitiveComponent Object Reference") (OtherBodyIndex :type Integer) (bFromSweep :type Boolean) (SweepResult :type "HitResult Structure (by ref)"))
  ;[1 1 1] On Collision
  (bind _asmmprojectile_base (cast `MMProjectileBase` OtherActor))
  (if (`|EnumInequality` (`MMProjectileBase.faction` _asmmprojectile_base) "Enemy")
    (bind _returnvalue (`|CreateWidget` "/Game/Blueprints/UI/ArenaChallengeUI/DamagePopUP.DamagePopUP_C"))
    (`UserWidget.AddToViewport` _returnvalue 0)
    (`/Game/Blueprints/UI/ArenaChallengeUI/DamagePopUP.Damage Text Pop Up Event` _returnvalue (`KismetMathLibrary.Round` (`MMProjectileBase.damage` _asmmprojectile_base)) (`GameplayStatics.ProjectWorldToScreen` (`GameplayStatics.GetPlayerController` 0) (`.ImpactPoint` (`GameplayStatics.BreakHitResult` SweepResult)) true))))

(fn `UserConstructionScript`)