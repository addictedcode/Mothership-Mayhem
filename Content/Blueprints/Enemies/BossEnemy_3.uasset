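; Boss enemy that performs charge, jump and ground slam attacks in arena fights.
; Unless winding up, Tick executes the current state: an interpolated lunge, a leap that teleports above the attack destination, or a rise and landing that spawns BP_Boss1Slam.
; Charge and jump damage the target by proximity.
; Projectile hits flash damage text or notify the boss game mode; death drops money and reports the kill to the arena game mode.
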(event `self.DeathGang`
  (`|SpawnActorFromClass` "/Game/Blueprints/Drops/MoneyDrop.MoneyDrop_C" (`KismetMathLibrary.Conv_VectorToTransform` (`self.K2_GetActorLocation` self)) "AdjustIfPossibleButAlwaysSpawn" "OverrideRootScale" null null)
  (cast `/Game/Blueprints/Characters/BP_MMCharacterBase` (`GameplayStatics.GetPlayerCharacter` 0))
  (bind _asmm_arena_game_mode (cast `/Game/Blueprints/Gamemodes/MM_ArenaGameMode` (`GameplayStatics.GetGameMode`)))
  (`/Game/Blueprints/Gamemodes/MM_ArenaGameMode.EnemyKilled` _asmm_arena_game_mode))

(event `self.CapsuleComponent.OnComponentHit`
  (params (HitComponent :type "PrimitiveComponent Object Reference") (OtherActor :type "Actor Object Reference") (OtherComp :type "PrimitiveComponent Object Reference") (NormalImpulse :type "Vector Structure") (Hit :type "HitResult Structure (by ref)"))
  (bind _asbp_mmprojectile_base (cast `/Game/Blueprints/Projectiles/BP_MMProjectileBase` OtherActor))
  (`TextRenderComponent.K2_SetText` (`self.TextRender`) (`KismetTextLibrary.Conv_DoubleToText` (`MMProjectileBase.damage` _asbp_mmprojectile_base) "HalfToEven"))
  (`KismetSystemLibrary.Delay` 0.2)
  (`TextRenderComponent.K2_SetText` (`self.TextRender`) (`KismetTextLibrary.Conv_StringToText` "")))

(event `self.Mesh.OnComponentHit`
  (params (HitComponent :type "PrimitiveComponent Object Reference") (OtherActor :type "Actor Object Reference") (OtherComp :type "PrimitiveComponent Object Reference") (NormalImpulse :type "Vector Structure") (Hit :type "HitResult Structure (by ref)"))
  (cast `MMProjectileBase` OtherActor)
  (bind _asmm_arena_game_mode_boss (cast `/Game/Blueprints/Gamemodes/MM_ArenaGameMode_Boss` (`GameplayStatics.GetGameMode`)))
  (`/Game/Blueprints/Gamemodes/MM_ArenaGameMode_Boss.Boss Hit` _asmm_arena_game_mode_boss (`self.K2_GetActorLocation`)))

(event `self.ReceiveTick`
  (params (DeltaSeconds :type "Float (single-precision)"))
  (bind _returnvalue (`self.K2_GetActorLocation`))
  (bind _returnvalue_2 (`self.K2_GetActorLocation`))
  (bind _returnvalue_3 (`self.K2_GetActorLocation`))
  (bind _returnvalue_4 (`self.K2_GetActorLocation`))
  ;[1 1 1] Raycast to floor
  (bind (_outhit _returnvalue_5) (`KismetSystemLibrary.LineTraceSingle` _returnvalue (`KismetMathLibrary.MakeVector` (.x _returnvalue) (.y _returnvalue) (- (.z _returnvalue) 10000.0)) "TraceTypeQuery1"))
  (if _returnvalue_5
    (set `self.DistanceToFloor` (`KismetMathLibrary.Vector_Distance` (`.Location` (`GameplayStatics.BreakHitResult` _outhit)) _returnvalue)))
  (`SceneComponent.K2_SetWorldRotation` (`self.TextRender`) (`KismetMathLibrary.Conv_VectorToRotator` (`KismetMathLibrary.GreaterGreater_VectorRotator` (`KismetMathLibrary.Normal` (* (- (`self.K2_GetActorLocation` (`GameplayStatics.GetPlayerPawn` 0)) (`SceneComponent.K2_GetComponentLocation` (`self.TextRender`))) (1.0 1.0 0.0))))) false false)
  (bind _returnvalue_6 (`self.GetWindingUp`))
  (if (not _returnvalue_6)
    (bind _returnvalue_7 (`self.GetCurrentState`))
    (switch `BossStates` _returnvalue_7
      (:`Charge`
        ;[1 1 1] Lunge
        (bind _returnvalue_8 (`self.GetAttackDestination`))
        (bind _returnvalue_9 (`KismetMathLibrary.VInterpTo` _returnvalue_2 (+ _returnvalue_8 (* (`KismetMathLibrary.Normal` (- _returnvalue_8 _returnvalue_2)) 1000.0)) DeltaSeconds 5.0))
        (`self.K2_SetActorLocation` _returnvalue_9 false true)
        (bind _returnvalue_10 (`self.GetTargetActor`))
        (if (<= (`KismetMathLibrary.Vector_Distance` (`self.K2_GetActorLocation` _returnvalue_10) _returnvalue_9) 100.0)
          (bind _asbp_mmcharacter_base (cast `/Game/Blueprints/Characters/BP_MMCharacterBase` _returnvalue_10))
          (`/Game/Blueprints/Characters/BP_MMCharacterBase.TakeDamage` _asbp_mmcharacter_base 40))
        (if (<= (`KismetMathLibrary.Vector_Distance` _returnvalue_9 _returnvalue_8) 100.0)
          (`self.ReturnToIdle`)))
      (:`JumpAttack`
        ;[1 1 1] Jump charge
        (bind _returnvalue_11 (`self.GetJumping`))
        (if _returnvalue_11
          (if (>= (.z (`self.K2_GetActorLocation`)) (`self.JumpAltitude`))
            (bind _returnvalue_12 (`self.GetAttackDestination`))
            (`self.K2_SetActorLocation` (+ _returnvalue_12 (`KismetMathLibrary.MakeVector` 0.0 0.0 (`self.JumpAltitude`))) false true)
            (`self.SetJumping` false)
            (else
              (`self.K2_SetActorLocation` (`KismetMathLibrary.VInterpTo` _returnvalue_4 (+ _returnvalue_4 (`KismetMathLibrary.MakeVector` 0.0 0.0 (`self.JumpAltitude`))) DeltaSeconds 5.0) false true)))
          (else
            (bind _returnvalue_13 (`self.GetTargetActor`))
            (if (<= (`KismetMathLibrary.Vector_Distance` (`self.K2_GetActorLocation` _returnvalue_13) (`self.K2_GetActorLocation`)) 100.0)
              (bind _asbp_mmcharacter_base_2 (cast `/Game/Blueprints/Characters/BP_MMCharacterBase` _returnvalue_13))
              (`/Game/Blueprints/Characters/BP_MMCharacterBase.TakeDamage` _asbp_mmcharacter_base_2 40))
            (if (not (`NavMovementComponent.IsFalling` (`self.CharacterMovement`)))
              (`self.ReturnToIdle`)))))
      (:`GroundSlam`
        ;[1 1 1] Ground Slam
        (bind _returnvalue_14 (`self.GetJumping`))
        (if _returnvalue_14
          (if (>= (.z (`self.K2_GetActorLocation`)) (`self.JumpAltitude`))
            (`self.SetJumping` false)
            (else
              (`self.K2_SetActorLocation` (`KismetMathLibrary.VInterpTo` _returnvalue_3 (+ _returnvalue_3 (`KismetMathLibrary.MakeVector` 0.0 0.0 (`self.JumpAltitude`))) DeltaSeconds 10.0) false true)))
          (elif (not (`NavMovementComponent.IsFalling` (`self.CharacterMovement`)))
            (bind _returnvalue_15 (`|SpawnActorFromClass` "/Game/Blueprints/Enemies/BP_Boss1Slam.BP_Boss1Slam_C" (`self.GetTransform`) "AdjustIfPossibleButAlwaysSpawn" "OverrideRootScale" null null))
            (`/Game/Blueprints/Enemies/BP_Boss1Slam.Activate` _returnvalue_15 (+ (`self.K2_GetActorLocation`) (`KismetMathLibrary.MakeVector` 0.0 0.0 -200.0)))
            (`self.ReturnToIdle`)))))))

(fn `UserConstructionScript`
  (`parent.UserConstructionScript`))