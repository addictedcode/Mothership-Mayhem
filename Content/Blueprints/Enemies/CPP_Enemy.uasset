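; Enemy actor Blueprint for an arena challenge, with death rewards and floating damage text.
; On DeathGang it spawns a MoneyDrop, decrements the enemy count on the player character's test arena UI reference and calls ClearLevel when none remain.
; Capsule hits from BP_MMProjectileBase briefly show the projectile's damage on a TextRender, which Tick turns horizontally toward the player.
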(event `self.DeathGang`
  (`|SpawnActorFromClass` "/Game/Blueprints/Drops/MoneyDrop.MoneyDrop_C" (`KismetMathLibrary.Conv_VectorToTransform` (`self.K2_GetActorLocation` self)) "AdjustIfPossibleButAlwaysSpawn" "OverrideRootScale" null null)
  (bind _asbp_mmcharacter_base (cast `/Game/Blueprints/Characters/BP_MMCharacterBase` (`GameplayStatics.GetPlayerCharacter` 0)))
  (bind _arenachallengeuiref_fortesting (`/Game/Blueprints/Characters/BP_MMCharacterBase.ArenaChallengeUIRef_FORTESTING` _asbp_mmcharacter_base))
  (bind _output_get (set `/Game/Blueprints/UI/ArenaChallengeUI/ArenaChallengePanelUI_FORTESTING.EnemyCount` (- (`/Game/Blueprints/UI/ArenaChallengeUI/ArenaChallengePanelUI_FORTESTING.EnemyCount` _arenachallengeuiref_fortesting) 1) _arenachallengeuiref_fortesting))
  (`KismetSystemLibrary.PrintString` (`KismetStringLibrary.Conv_IntToString` _output_get))
  (if (<= _output_get 0)
    (`/Game/Blueprints/UI/ArenaChallengeUI/ArenaChallengePanelUI_FORTESTING.ClearLevel` _arenachallengeuiref_fortesting)
    (`/Game/Blueprints/UI/ArenaChallengeUI/ArenaChallengePanelUI_FORTESTING.ClearLevel` _arenachallengeuiref_fortesting)))

(event `self.ReceiveTick`
  (params (DeltaSeconds :type "Float (single-precision)"))
  (`SceneComponent.K2_SetWorldRotation` (`self.TextRender`) (`KismetMathLibrary.Conv_VectorToRotator` (`KismetMathLibrary.GreaterGreater_VectorRotator` (`KismetMathLibrary.Normal` (* (- (`self.K2_GetActorLocation` (`GameplayStatics.GetPlayerPawn` 0)) (`SceneComponent.K2_GetComponentLocation` (`self.TextRender`))) (1.0 1.0 0.0))))) false false))

(event `self.CapsuleComponent.OnComponentHit`
  (params (HitComponent :type "PrimitiveComponent Object Reference") (OtherActor :type "Actor Object Reference") (OtherComp :type "PrimitiveComponent Object Reference") (NormalImpulse :type "Vector Structure") (Hit :type "HitResult Structure (by ref)"))
  (bind _asbp_mmprojectile_base (cast `/Game/Blueprints/Projectiles/BP_MMProjectileBase` OtherActor))
  (`TextRenderComponent.K2_SetText` (`self.TextRender`) (`KismetTextLibrary.Conv_DoubleToText` (`MMProjectileBase.damage` _asbp_mmprojectile_base) "HalfToEven"))
  (`KismetSystemLibrary.Delay` 0.2)
  (`TextRenderComponent.K2_SetText` (`self.TextRender`) (`KismetTextLibrary.Conv_StringToText` "")))

(fn `UserConstructionScript`)