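; BP_ElectricFence is a hazard actor that knocks back and damages characters that hit its Box collider.
; On hit, it launches the character along the Arrow component's forward vector with a slight upward tilt, using a velocity-change impulse on CharacterMovement.
; BP_MMCharacterBase takes DamageDealt directly, while AICharacter takes it through its EnemyStats; other actors are ignored.
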(event `self.Box.OnComponentHit`
  (params (HitComponent :type "PrimitiveComponent Object Reference") (OtherActor :type "Actor Object Reference") (OtherComp :type "PrimitiveComponent Object Reference") (NormalImpulse :type "Vector Structure") (Hit :type "HitResult Structure (by ref)"))
  (bind _asbp_mmcharacter_base (cast `/Game/Blueprints/Characters/BP_MMCharacterBase` OtherActor)
    (:`then`
      (`CharacterMovementComponent.AddImpulse` (`Character.CharacterMovement` _asbp_mmcharacter_base) (* (`KismetMathLibrary.Normal` (+ (`SceneComponent.GetForwardVector` (`self.Arrow`)) (0.0 0.0 0.1))) 2000.0) true)
      (`/Game/Blueprints/Characters/BP_MMCharacterBase.TakeDamage` _asbp_mmcharacter_base (`self.DamageDealt`)))
    (:`CastFailed`
      (bind _asaicharacter (cast `AICharacter` OtherActor))
      (`CharacterMovementComponent.AddImpulse` (`Character.CharacterMovement` _asaicharacter) (* (`KismetMathLibrary.Normal` (+ (`SceneComponent.GetForwardVector` (`self.Arrow`)) (0.0 0.0 0.1))) 2000.0) true)
      (bind _returnvalue (`AICharacter.getEnemyStats` _asaicharacter))
      (`EnemyStatsComponent.TakeDamage` _returnvalue (`self.DamageDealt`)))))

(fn `UserConstructionScript`)