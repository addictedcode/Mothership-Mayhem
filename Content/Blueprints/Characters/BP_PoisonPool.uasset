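; BP_PoisonPool is a temporary damage-over-time area that hurts characters and enemies standing inside it.
; Tick counts up its lifetime and, at a fixed interval, polls the actors overlapping its box detector.
; Player-side BP_MMCharacterBase actors take damage directly, while CPP_Enemy actors take it through their enemy stats.
; Once the active duration runs out, the pool destroys itself.
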(event `self.ReceiveTick`
  (params (DeltaSeconds :type "Float (single-precision)"))
  (bind _damage_dealt (`self.Damage Dealt`))
  (bind _output_get (set `self.CurretActiveTime` (+ DeltaSeconds (`self.CurretActiveTime`))))
  (if (< _output_get (`self.ActiveDuration`))
    (bind _output_get_2 (set `self.TimeSinceLastTick` (+ DeltaSeconds (`self.TimeSinceLastTick`))))
    (if (>= _output_get_2 (`self.TimePerTick`))
      (set `self.TimeSinceLastTick` 0.0)
      (for _array_element (`PrimitiveComponent.GetOverlappingActors` (`self.BoxDetector`) null)
        (bind _asbp_mmcharacter_base (cast `/Game/Blueprints/Characters/BP_MMCharacterBase` _array_element)
          (:`then`
            (`/Game/Blueprints/Characters/BP_MMCharacterBase.TakeDamage` _asbp_mmcharacter_base _damage_dealt))
          (:`CastFailed`
            (bind _ascpp_enemy (cast `/Game/Blueprints/Enemies/CPP_Enemy` _array_element))
            (bind _returnvalue (`AICharacter.getEnemyStats` _ascpp_enemy))
            (`EnemyStatsComponent.TakeDamage` _returnvalue _damage_dealt)))))
    (else
      (`self.K2_DestroyActor`))))

(fn `UserConstructionScript`)