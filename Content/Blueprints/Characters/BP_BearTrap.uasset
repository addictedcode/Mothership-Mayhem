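; BP_BearTrap is a single-use trap actor that damages and shocks the first enemy to step into it.
; A BoxDetector overlap casts to CPP_Enemy, then uses its EnemyStats to deal DamageDealt and apply the SHOCKING status before destroying the trap.
; Tick accumulates lifetime and destroys an untriggered trap once ActiveDuration elapses.
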(event `self.ReceiveTick`
  (params (DeltaSeconds :type "Float (single-precision)"))
  (bind _output_get (set `self.CurretActiveTime` (+ DeltaSeconds (`self.CurretActiveTime`))))
  (if (not (< _output_get (`self.ActiveDuration`)))
    (`self.K2_DestroyActor` :!label _label)))

(event `self.BoxDetector.OnComponentBeginOverlap`
  (params (OverlappedComponent :type "PrimitiveComponent Object Reference") (OtherActor :type "Actor Object Reference") (OtherComp :type "PrimitiveComponent Object Reference") (OtherBodyIndex :type Integer) (bFromSweep :type Boolean) (SweepResult :type "HitResult Structure (by ref)"))
  (bind _ascpp_enemy (cast `/Game/Blueprints/Enemies/CPP_Enemy` OtherActor))
  (bind _returnvalue (`AICharacter.getEnemyStats` _ascpp_enemy))
  (`EnemyStatsComponent.TakeDamage` _returnvalue (`self.Damage Dealt`))
  (`EnemyStatsComponent.ApplyStatusEffect` _returnvalue "SHOCKING")
  (goto _label))

(fn `UserConstructionScript`)