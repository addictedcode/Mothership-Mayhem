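; Base character Blueprint that puts the mod shop UI on screen and lets the player interact with objects in front of the camera.
; On BeginPlay it creates the ModShopUI widget, stores a reference and adds it to the viewport.
; The Interact input runs a short object-type line trace along the camera's facing.
; A hit box component attached to an InteractableComponent causes that parent component to be triggered.
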(event `self.ReceiveBeginPlay`
  (bind _returnvalue (`|CreateWidget` "/Game/Blueprints/UI/ModShop/ModShopUI.ModShopUI_C"))
  (bind _output_get (set `self.ModShopUIReference` _returnvalue))
  (`UserWidget.AddToViewport` _output_get 0))

(event `InputAction|Interact`
  (params (Key :type "Key Structure"))
  (bind _cameracomponent (`self.cameraComponent`))
  (bind _returnvalue (`SceneComponent.K2_GetComponentLocation` _cameracomponent))
  (:`Pressed`
    (bind (_outhit _returnvalue_2) (`KismetSystemLibrary.LineTraceSingleForObjects` _returnvalue (+ _returnvalue (`KismetMathLibrary.GreaterGreater_VectorRotator` (`KismetMathLibrary.MakeVector` 200.0) (`SceneComponent.K2_GetComponentRotation` _cameracomponent))) (`|MakeArray` "ObjectTypeQuery1" "ObjectTypeQuery2" :!type "EObjectTypeQuery Enum")))
    (if _returnvalue_2
      (bind _asbox_collision (cast `BoxComponent` (`.HitComponent` (`GameplayStatics.BreakHitResult` _outhit))))
      (bind _asinteractable_component (cast `InteractableComponent` (`SceneComponent.GetAttachParent` _asbox_collision)))
      (`InteractableComponent.Trigger` _asinteractable_component null))))

(fn `UserConstructionScript`)