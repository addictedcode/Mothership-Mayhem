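; Destructible prop that bursts apart and drops gear money pickups when it breaks.
; On component fracture, it applies a constant-falloff radial force just above the Destructible component to scatter the pieces.
; It then spawns MoneyDrops in a GearCount-driven loop at slightly randomized offsets, nudging each gear mesh with a randomized, upward-biased force.
; The HasMoneySpawned flag limits drops to the first fracture, while the radial force repeats on every fracture event.
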(event `self.Destructible.OnComponentFracture`
  (params (HitPoint :type "Vector Structure (by ref)") (HitDirection :type "Vector Structure (by ref)"))
  (bind _destructible (`self.Destructible`))
  (`PrimitiveComponent.AddRadialForce` _destructible (+ (`SceneComponent.K2_GetComponentLocation` _destructible) (0.0 0.0 50.0)) 100.0 1000.0 "RIF_Constant" false)
  (if (not (`self.hasMoneySpawned`))
    (for _ (range (+ (`self.GearCount`) 1))
      (bind _returnvalue (`|SpawnActorFromClass` "/Game/Blueprints/Drops/MoneyDrops.MoneyDrops_C" (`KismetMathLibrary.Conv_VectorToTransform` (+ (`SceneComponent.K2_GetComponentLocation` (`self.Destructible`)) (`KismetMathLibrary.MakeVector` (`KismetMathLibrary.RandomFloatInRange` 0.0 10.0) (`KismetMathLibrary.RandomFloatInRange` 0.0 10.0) 50.0))) "Undefined" "OverrideRootScale" null null))
      (`PrimitiveComponent.AddForce` (`/Game/Blueprints/Drops/MoneyDrops.GearMesh` _returnvalue) (`KismetMathLibrary.MakeVector` (`KismetMathLibrary.RandomFloatInRange` 0.0 20.0) (`KismetMathLibrary.RandomFloatInRange` 0.0 20.0) 50.0) "None" false)
      (set `self.hasMoneySpawned` true))))

(fn `UserConstructionScript`)