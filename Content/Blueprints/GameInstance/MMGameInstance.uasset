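; Game instance that holds the player's fame progression and the mods equipped on their guns.
; Fame points are clamped to the current rank's threshold, and reaching it allows a rank up that zeroes the points.
; Mod lists for three gun slots are copied from the character's gun loadout component into instance arrays, and re-added to the guns after a pass that removes their current mods.
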(fn `CanRankUp`
  (returns (CanRankUp :type Boolean))
  (return (== (`self.FamePoints`) (`|GetArrayItem` (`self.PointsToRankUp`) (- (`self.FameRank`) 1)))))

(fn `GainFame`
  (params (Increase :type Integer))
  (set `self.FamePoints` (`KismetMathLibrary.Clamp` (+ Increase (`self.FamePoints`)) 0 (`|GetArrayItem` (`self.PointsToRankUp`) (- (`self.FameRank`) 1)))))

(fn `RankUp`
  (bind _canrankup (`self.CanRankUp`))
  (if _canrankup
    (set `self.FameRank` (+ (`self.FameRank`) 1))
    (set `self.FamePoints` 0)))

(fn `ResetRank`
  (set `self.FameRank` 1)
  (set `self.FamePoints` 0))

(fn `SetRank`
  (params (Rank :type Integer) (Points :type Integer))
  (set `self.FameRank` Rank)
  (set `self.FamePoints` Points))

(fn `Update Char Mods`
  (bind _asbp_mmcharacter_base (cast `/Game/Blueprints/Characters/BP_MMCharacterBase` (`GameplayStatics.GetPlayerCharacter` 0)))
  (bind _returnvalue (`MMGunLoadout.getGuns` (`MMCharacterBase.gunLoadoutComponent` _asbp_mmcharacter_base)))
  (for (_array_element _array_index) _returnvalue
    (bind _returnvalue_2 (`MMGunBase.GetModList` _array_element))
    ;[1 1 1] Removes all the Mods of the Gun
    (for _ _returnvalue_2
      (`MMGunBase.RemoveModByIndex` _array_element (`KismetArrayLibrary.Array_Length` _returnvalue_2)))
    (switch `int` _array_index
      (:`0`
        ;[1 1 1] Adds Mods back into gun
        (for _array_element_2 (`self.ModsEquipped_Gun0`)
          (`MMGunBase.AddMod` _array_element _array_element_2)))
      (:`1`
        (for _array_element_3 (`self.ModsEquipped_Gun1`)
          (`MMGunBase.AddMod` _array_element _array_element_3)))
      (:`2`
        (for _array_element_4 (`self.ModsEquipped_Gun2`)
          (`MMGunBase.AddMod` _array_element _array_element_4))))))

(fn `Update Instance Mods`
  (bind _asbp_mmcharacter_base (cast `/Game/Blueprints/Characters/BP_MMCharacterBase` (`GameplayStatics.GetPlayerCharacter` 0)))
  ;[1 1 1] Adds Mods from gun to Game Instance Mod Arrays
  (bind _returnvalue (`MMGunLoadout.getGuns` (`MMCharacterBase.gunLoadoutComponent` _asbp_mmcharacter_base)))
  (for (_array_element _array_index) _returnvalue
    (switch `int` _array_index
      (:`0`
        (bind _returnvalue_2 (`MMGunBase.GetModList` _array_element))
        (bind _output_get (set `self.ModsEquipped_Gun0` _returnvalue_2))
        (for _ _output_get
          _))
      (:`1`
        (bind _output_get_2 (set `self.ModsEquipped_Gun1` _returnvalue_2))
        (for _ _output_get_2
          _))
      (:`2`
        (bind _output_get_3 (set `self.ModsEquipped_Gun2` _returnvalue_2))
        (for _ _output_get_3
          _)))))