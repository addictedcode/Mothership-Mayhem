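; Machine gun Blueprint that supplies the weapon's recoil and reload visuals on its skeletal gun mesh.
; The recoil event plays the recoil animation and spawns a muzzle flash effect at the MuzzlePoint socket, storing the spawned component.
; The reload event plays the reload animation and sets its play rate to the inverse of the ReloadTime from the gun's final stats.
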(event `self.PlayRecoilAnimation`
  (`SkeletalMeshComponent.PlayAnimation` (`self.skeletalGunMesh`) "/Game/Assets/Models/Guns/MachineGun/MachineGun_Recoil.MachineGun_Recoil" false)
  (bind _returnvalue (`NiagaraFunctionLibrary.SpawnSystemAtLocation` (`self.muzzleFlashFX`) (.location (`SceneComponent.GetSocketTransform` (`self.skeletalGunMesh`) "MuzzlePoint" "RTS_World")) (.rotation (`SceneComponent.GetSocketTransform` (`self.skeletalGunMesh`) "MuzzlePoint" "RTS_World"))))
  (set `self.muzzleFlash` _returnvalue))

(event `self.PlayReloadAnimation`
  (bind _skeletalgunmesh (`self.skeletalGunMesh`))
  (`SkeletalMeshComponent.PlayAnimation` _skeletalgunmesh "/Game/Assets/Models/Guns/MachineGun/MachineGun_BetterReload.MachineGun_BetterReload" false)
  (bind _returnvalue (`self.GetFinalStats`))
  (`SkeletalMeshComponent.SetPlayRate` _skeletalgunmesh (/ 1.0 (`.reloadTime` (break `GunStats` _returnvalue)))))

(fn `UserConstructionScript`)