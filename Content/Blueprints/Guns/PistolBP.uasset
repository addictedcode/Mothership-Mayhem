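; Pistol gun Blueprint that supplies the weapon's recoil and reload visuals.
; The recoil event plays the recoil animation on the skeletal gun mesh and spawns a muzzle flash effect at the MuzzlePoint socket's world location and rotation.
; The reload event plays the reload animation and sets its play rate to the inverse of ReloadTime from GetFinalStats, so playback speed follows the gun's final stats.
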(event `self.PlayRecoilAnimation`
  (`SkeletalMeshComponent.PlayAnimation` (`self.skeletalGunMesh`) "/Game/Assets/Models/Guns/Pistol/Pistol_Recoil_Anim.Pistol_Recoil_Anim" false)
  (`NiagaraFunctionLibrary.SpawnSystemAtLocation` (`self.muzzleFlashFX`) (.location (`SceneComponent.GetSocketTransform` (`self.skeletalGunMesh`) "MuzzlePoint" "RTS_World")) (.rotation (`SceneComponent.GetSocketTransform` (`self.skeletalGunMesh`) "MuzzlePoint" "RTS_World"))))

(event `self.PlayReloadAnimation`
  (bind _skeletalgunmesh (`self.skeletalGunMesh`))
  (`SkeletalMeshComponent.PlayAnimation` _skeletalgunmesh "/Game/Assets/Models/Guns/Pistol/Pistol_Reload_Anim.Pistol_Reload_Anim" false)
  (bind _returnvalue (`self.GetFinalStats`))
  (`SkeletalMeshComponent.SetPlayRate` _skeletalgunmesh (/ 1.0 (`.reloadTime` (break `GunStats` _returnvalue)))))

(fn `UserConstructionScript`)