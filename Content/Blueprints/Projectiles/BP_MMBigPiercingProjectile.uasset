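; Big piercing projectile Blueprint that damages AI characters it overlaps, with no destroy logic in this graph.
; Collision overlap plays a hit sound at world origin, spawns a pierce Niagara effect at the sweep location, then applies its damage value through the character's enemy stats.
; A separate Hit event plays the same sound and effect at the hit location without damage.
; An alternate damage path via the overlapped component's owner is disconnected.
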(event `self.ReceiveHit`
  (params (MyComp :type "PrimitiveComponent Object Reference") (Other :type "Actor Object Reference") (OtherComp :type "PrimitiveComponent Object Reference") (bSelfMoved :type Boolean) (HitLocation :type "Vector Structure") (HitNormal :type "Vector Structure") (NormalImpulse :type "Vector Structure") (Hit :type "HitResult Structure (by ref)"))
  (`GameplayStatics.PlaySoundAtLocation` "/Game/Assets/Audio/GunHitSound.GunHitSound" HitLocation (struct) 1.0 1.0 0.0 null null null)
  (`NiagaraFunctionLibrary.SpawnSystemAtLocation` "/Game/Assets/ParticleFX/ProjectileOnHitEffects/NE_System_PierceOnHit.NE_System_PierceOnHit" HitLocation))

(event `self.collisionComp.OnComponentBeginOverlap`
  (params (OverlappedComponent :type "PrimitiveComponent Object Reference") (OtherActor :type "Actor Object Reference") (OtherComp :type "PrimitiveComponent Object Reference") (OtherBodyIndex :type Integer) (bFromSweep :type Boolean) (SweepResult :type "HitResult Structure (by ref)"))
  (`|ExecutionSequence`
    (:`then_0`
      (`GameplayStatics.PlaySoundAtLocation` "/Game/Assets/Audio/GunHitSound.GunHitSound" (0.0 0.0 0.0) (struct) 1.0 1.0 0.0 null null null)
      (`NiagaraFunctionLibrary.SpawnSystemAtLocation` "/Game/Assets/ParticleFX/ProjectileOnHitEffects/NE_System_PierceOnHit.NE_System_PierceOnHit" (`.Location` (`GameplayStatics.BreakHitResult` SweepResult))))
    (:`then_1`
      (bind _asaicharacter (cast `AICharacter` OtherActor))
      (bind _returnvalue (`AICharacter.getEnemyStats` _asaicharacter))
      (bind _returnvalue_2 (`self.getDamageValue`))
      (`EnemyStatsComponent.TakeDamage` _returnvalue _returnvalue_2))))

(fn `UserConstructionScript`)