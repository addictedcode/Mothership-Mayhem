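; Projectile Blueprint that bursts into gear sub-projectiles when it hits.
; On Hit it plays a hit sound at the world origin and spawns an impact effect at the hit point.
; If its parent is a ProjectilePool, two loops spawn BP_gearSubProjectile through that pool at the hit point.
; Directions step around Z from the actor's right vector, with the second ring tilted by a further 90-degree rotation.
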(event `self.ReceiveHit`
  (params (MyComp :type "PrimitiveComponent Object Reference") (Other :type "Actor Object Reference") (OtherComp :type "PrimitiveComponent Object Reference") (bSelfMoved :type Boolean) (HitLocation :type "Vector Structure") (HitNormal :type "Vector Structure") (NormalImpulse :type "Vector Structure") (Hit :type "HitResult Structure (by ref)"))
  (`GameplayStatics.PlaySoundAtLocation` "/Game/Assets/Audio/GunHitSound.GunHitSound" (0.0 0.0 0.0) (struct) 1.0 1.0 0.0 null null null)
  (`NiagaraFunctionLibrary.SpawnSystemAtLocation` "/Game/Assets/Animations/Pistol/BulletHit_FX.BulletHit_FX" HitLocation)
  (bind _asprojectile_pool (cast `ProjectilePool` (`self.parentPool`)))
  (for _index (range 11)
    (`ProjectilePool.SpawnObjectWDefaultSpawnParams` _asprojectile_pool "/Game/Blueprints/Projectiles/SubProjectiles/BP_gearSubProjectile.BP_gearSubProjectile_C" HitLocation (`KismetMathLibrary.Conv_VectorToRotator` (`KismetMathLibrary.RotateAngleAxis` (`self.GetActorRightVector`) (* _index 36.0) (0.0 0.0 1.0)))))
  (for _index_2 (range 11)
    (`ProjectilePool.SpawnObjectWDefaultSpawnParams` _asprojectile_pool "/Game/Blueprints/Projectiles/SubProjectiles/BP_gearSubProjectile.BP_gearSubProjectile_C" HitLocation (`KismetMathLibrary.Conv_VectorToRotator` (`KismetMathLibrary.RotateAngleAxis` (`KismetMathLibrary.RotateAngleAxis` (`self.GetActorRightVector`) (* _index_2 36.0) (0.0 0.0 1.0)) 90.0 (0.0 1.0 1.0))))))

(fn `UserConstructionScript`)