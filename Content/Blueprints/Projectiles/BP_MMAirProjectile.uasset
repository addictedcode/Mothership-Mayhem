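; BP_MMAirProjectile is an air projectile that pushes AI characters it hits.
; On hit, it spawns a Niagara effect at the impact point and plays a hit sound at the world origin.
; If the target is an AICharacter, it applies a velocity-change impulse along the projectile's horizontal forward direction with slight lift, scaled by PushStrength.
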(event `self.ReceiveHit`
  (params (MyComp :type "PrimitiveComponent Object Reference") (Other :type "Actor Object Reference") (OtherComp :type "PrimitiveComponent Object Reference") (bSelfMoved :type Boolean) (HitLocation :type "Vector Structure") (HitNormal :type "Vector Structure") (NormalImpulse :type "Vector Structure") (Hit :type "HitResult Structure (by ref)"))
  (`GameplayStatics.PlaySoundAtLocation` "/Game/Assets/Audio/GunHitSound.GunHitSound" (0.0 0.0 0.0) (struct) 1.0 1.0 0.0 null null null)
  (`NiagaraFunctionLibrary.SpawnSystemAtLocation` "/Game/Assets/ParticleFX/projectileOnHit1_System.projectileOnHit1_System" HitLocation)
  (bind _asaicharacter (cast `AICharacter` Other))
  (`CharacterMovementComponent.AddImpulse` (`Character.CharacterMovement` _asaicharacter) (* (`KismetMathLibrary.Normal` (`KismetMathLibrary.MakeVector` (.x (`self.GetActorForwardVector`)) (.y (`self.GetActorForwardVector`)) 0.1)) (`self.Push Strength`)) true))

(fn `UserConstructionScript`)