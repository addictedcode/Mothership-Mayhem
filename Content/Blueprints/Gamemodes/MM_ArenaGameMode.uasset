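; Arena game mode that runs the challenge stored in MMGameInstance and opens MM_Spaceship on a win or loss.
; Extermination spawns every wave at start and wins when the kill count empties.
; Survival counts down on Tick, spawning cycled waves at cooldown multiples and checking for victory only while spawning.
; One EnemySpawner is teleported to random points in round-robin zone boxes; Defense only handles results, losing when its pod is destroyed.
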(event `self.ReceiveBeginPlay`
  (bind _spawner (`self.Spawner`))
  (bind _spawnzone (`self.spawnZone`))
  (`parent.ReceiveBeginPlay`)
  (`|ExecutionSequence`
    (:`then_0`
      ;[1 1 1] Initialization
      ;;[1 1 1] Arena Challenge
      (bind _asmmgame_instance (cast `/Game/Blueprints/GameInstance/MMGameInstance` (`GameplayStatics.GetGameInstance`)))
      (bind _current_arena_challenge (`/Game/Blueprints/GameInstance/MMGameInstance.current Arena Challenge` _asmmgame_instance))
      (set `self.Current Arena Challenge` _current_arena_challenge)
      (set `self.Current Challenge Type` (`MMArenaChallenge_DataAsset.challengeType` _current_arena_challenge))
      (set `self.time` (`KismetMathLibrary.Conv_IntToDouble` (`MMArenaChallenge_DataAsset.timeLimitSeconds` _current_arena_challenge)))
      ;;[1 1 1] Spawn Zone
      (bind _outactors (`GameplayStatics.GetAllActorsOfClass` "/Game/Blueprints/spawnZoneTest.spawnZoneTest_C"))
      (for _array_element _outactors
        (`KismetArrayLibrary.Array_Add` (`self.spawnZoneArray`) (`self.GetComponentByClass` _array_element "/Script/Engine.BoxComponent"))
        ;;[1 1 1] Spawner
        (bind _returnvalue (`GameplayStatics.GetActorOfClass` "/Script/MothershipMayhem.EnemySpawner"))
        (set `self.Spawner` _returnvalue)))
    (:`then_1`
      (switch `MMChallengeType` (`self.Current Challenge Type`)
        (:`Survival`
          ;[1 1 1] Survival Challenge
          (`KismetSystemLibrary.PrintString` "Survival Challenge!"))
        (:`Extermination`
          ;[1 1 1] Extermination
          (`KismetSystemLibrary.PrintString` "Extermination Challenge!")
          (set `self.EnemyCount` 0)
          (for _array_element_2 (`MMArenaChallenge_DataAsset.spawnList` (`self.Current Arena Challenge`))
            (`self.ChooseSpawnZone`)
            (for _array_element_3 (`MMEnemyWave_DataAsset.spawnList` _array_element_2)
              ;;[1 1 1] Spawning
              (set `EnemySpawner.ActorToSpawn` _array_element_3 _spawner)
              (`self.K2_SetActorLocation` _spawner (`KismetMathLibrary.RandomPointInBoundingBox` (`SceneComponent.K2_GetComponentLocation` _spawnzone) (`BoxComponent.GetScaledBoxExtent` _spawnzone)) false true)
              (`EnemySpawner.SpawnEnemy` _spawner)
              (set `self.EnemyCount` (+ (`self.EnemyCount`) 1))))
          (`KismetSystemLibrary.PrintString` (`KismetStringLibrary.Conv_IntToString` (`self.EnemyCount`))))))))

(event `self.ReceiveTick`
  (params (DeltaSeconds :type "Float (single-precision)"))
  (bind _spawner (`self.Spawner`))
  (bind _spawnzone (`self.spawnZone`))
  (switch `MMChallengeType` (`self.Current Challenge Type`)
    (:`Survival`
      ;[1 1 1] Survival
      (`|ExecutionSequence`
        (:`then_0`
          ;;[1 1 1] Timer
          (bind _output_get (set `self.time` (- (`self.time`) DeltaSeconds)))
          (bind _returnvalue (`KismetMathLibrary.Round` _output_get))
          (if (!= (`self.display time`) _returnvalue)
            (bind _output_get_2 (set `self.display time` _returnvalue))
            (`KismetSystemLibrary.PrintString` (`KismetStringLibrary.Conv_IntToString` _output_get_2))
            (if (== (mod _output_get_2 (`self.respawnCooldown`)) 0)
              (`KismetSystemLibrary.PrintString` "SPAWN")
              ;;[1 1 1] Spawning
              (`self.ChooseSpawnZone`)
              (`self.choose Survival wave`)
              (for _array_element (`MMEnemyWave_DataAsset.spawnList` (`|GetArrayItem` (`MMArenaChallenge_DataAsset.spawnList` (`self.Current Arena Challenge`)) (`self.currentWave`)))
                (set `EnemySpawner.ActorToSpawn` _array_element _spawner)
                (`self.K2_SetActorLocation` _spawner (`KismetMathLibrary.RandomPointInBoundingBox` (`SceneComponent.K2_GetComponentLocation` _spawnzone) (`BoxComponent.GetScaledBoxExtent` _spawnzone)) false true)
                (`EnemySpawner.SpawnEnemy` _spawner)
                ;;[1 1 1] WIN CONDITION
                (if (<= (`self.time`) 0.0)
                  (`self.WinArenaChallenge`))))))))))

(event `WinArenaChallenge`
  ;[1 1 1] Win
  (switch `MMChallengeType` (`self.Current Challenge Type`)
    (:`Survival`
      (`KismetSystemLibrary.PrintString` "YOU SURVIVED")
      (`GameplayStatics.OpenLevel` "MM_Spaceship"))
    (:`Defense`
      (`KismetSystemLibrary.PrintString` "YOU DEFENDED")
      (`GameplayStatics.OpenLevel` "MM_Spaceship"))
    (:`Extermination`
      (`KismetSystemLibrary.PrintString` "YOU EXTERMINATED")
      (`GameplayStatics.OpenLevel` "MM_Spaceship"))))

(event `Lose Arena Challenge`
  (switch `MMChallengeType` (`self.Current Challenge Type`)
    (:`Survival`
      (`KismetSystemLibrary.PrintString` "You unsurvived"))
    (:`Defense`
      (`KismetSystemLibrary.PrintString` "you undefended"))
    (:`Extermination`
      (`KismetSystemLibrary.PrintString` "you got exterminated!")))
  (`GameplayStatics.OpenLevel` "MM_Spaceship"))

(event `EnemyKilled`
  ;[1 1 1] Extermination: Enemy Killed
  (bind _result (`/Engine/EditorBlueprintResources/StandardMacros.DecrementInt` (`self.EnemyCount`))
    (:`  `
      (bind _output_get (set `self.EnemyCount` _result))
      (if (<= _output_get 0)
        (switch `MMChallengeType` (`self.Current Challenge Type`)
          (:`Extermination`
            (`self.WinArenaChallenge`)))
        (else
          (`KismetSystemLibrary.PrintString` (`KismetStringLibrary.Conv_IntToString` _output_get)))))))

(event `DefensePodDestroyed`
  ;[1 1 1] Defense: Defense Pod Destroyed
  (`self.Lose Arena Challenge`))

(fn `choose Survival wave`
  (bind _returnvalue (+ (`self.currentWave`) 1))
  (if (>= _returnvalue (`KismetArrayLibrary.Array_Length` (`MMArenaChallenge_DataAsset.spawnList` (`self.Current Arena Challenge`))))
    (set `self.currentWave` 0)
    (return)
    (else
      (set `self.currentWave` _returnvalue)
      (return))))

(fn `ChooseSpawnZone`
  (if (>= (+ (`self.currentSpawnZone`) 1) (`KismetArrayLibrary.Array_Length` (`self.spawnZoneArray`)))
    (set `self.currentSpawnZone` 0)
    (set `self.spawnZone` (`|GetArrayItem` (`self.spawnZoneArray`) (`self.currentSpawnZone`)))
    (return)
    (else
      (set `self.currentSpawnZone` (+ (`self.currentSpawnZone`) 1))
      (set `self.spawnZone` (`|GetArrayItem` (`self.spawnZoneArray`) (`self.currentSpawnZone`)))
      (return))))

(fn `SpawnWave`)

(fn `Survival`
  (params (deltaSeconds :type "Float (double-precision)")))

(fn `UserConstructionScript`
  (`parent.UserConstructionScript`))