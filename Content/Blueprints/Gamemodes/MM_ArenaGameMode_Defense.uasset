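; Arena game mode for Defense challenges, where the player protects a DefensePod until a timer runs out.
; BeginPlay finds the pod, switches the player to the Defense HUD and shows a tutorial popup on low difficulties.
; Tick counts down and periodically moves a spawner within a chosen zone to spawn waves, retargeting pooled enemies at the pod.
; Once time is up and no enemies remain, the challenge is won with pod-generated scraps as bonus.
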(event `self.ReceiveBeginPlay`
  (`parent.ReceiveBeginPlay`)
  (bind _returnvalue (`GameplayStatics.GetActorOfClass` "/Game/Blueprints/Interactables/DefensePod.DefensePod_C"))
  (set `self.Defense Pod` _returnvalue)
  ;[1 1 1] UI
  (`KismetSystemLibrary.Delay` 0.2)
  (bind _asbp_mmcharacter_base (cast `/Game/Blueprints/Characters/BP_MMCharacterBase` (`GameplayStatics.GetPlayerCharacter` 0)))
  (`/Game/Blueprints/UI/ArenaChallengeUI/DefenseHUD.Activate Defense HUD UI` (`/Game/Blueprints/Characters/BP_MMCharacterBase.DefenseHUDUIReference` _asbp_mmcharacter_base))
  (`/Game/Blueprints/UI/ArenaChallengeUI/ExterminationHUD.Deactivate Extermination HUD UI` (`/Game/Blueprints/Characters/BP_MMCharacterBase.ExterminationHUDUIReference` _asbp_mmcharacter_base))
  (`/Game/Blueprints/UI/ArenaChallengeUI/SurvivalHUD.Deactivate Survival HUD UI` (`/Game/Blueprints/Characters/BP_MMCharacterBase.SurvivalHUDUIReference` _asbp_mmcharacter_base))
  (`KismetSystemLibrary.PrintString` (`KismetStringLibrary.Conv_IntToString` (`/Game/Blueprints/UI/HUD/HUD.Max HP` (`/Game/Blueprints/Characters/BP_MMCharacterBase.HUDUIReference` _asbp_mmcharacter_base))))
  (if (<= (`MMArenaChallenge_DataAsset.difficultyLevel` (`self.currentArenaChallenge`)) 2)
    (set `self.isTutorial` true)
    (`KismetSystemLibrary.Delay` 0.2)
    (bind _asbp_mmcharacter_base_2 (cast `/Game/Blueprints/Characters/BP_MMCharacterBase` (`GameplayStatics.GetPlayerCharacter` 0)))
    (`/Game/Blueprints/UI/HUD/HUD.OpenPopUp` (`/Game/Blueprints/Characters/BP_MMCharacterBase.HUDUIReference` _asbp_mmcharacter_base_2) "This is the Defense Game Mode!   \nYour goal is to defend the pod until the timer ends. \nThe Energy Meter in the top left dictates the rate that scraps (used in the shop) are generated. This meter depletes over time. Killing enemies drops materials that can be used to energize the pod, or to repair it, bring it to either robot to dump the materials into the generator for energy or repair.")
    (else
      (set `self.isTutorial` false))))

(event `self.ReceiveTick`
  (params (DeltaSeconds :type "Float (single-precision)"))
  (bind _spawner (`self.Spawner`))
  (bind _display_time (`self.display time`))
  (bind _spawnzone (`self.spawnZone`))
  (bind _generatedmoney (`/Game/Blueprints/Interactables/DefensePod.GeneratedMoney` (`self.Defense Pod`)))
  (`parent.ReceiveTick` DeltaSeconds)
  (`|ExecutionSequence`
    (:`then_0`
      (if (<= (`self.EnemyCount`) 0)
        (if (<= (`self.time`) 0.0)
          (`KismetSystemLibrary.PrintString` (`KismetStringLibrary.Conv_DoubleToString` _generatedmoney))
          (`self.WinArenaChallenge` 1.0 (`KismetMathLibrary.FTrunc` _generatedmoney)))))
    (:`then_1`
      ;[1 1 1] Defense
      (`|ExecutionSequence`
        (:`then_0`
          ;;[1 1 1] Timer
          (bind _output_get (set `self.time` (- (`self.time`) DeltaSeconds)))
          (bind _returnvalue (`KismetMathLibrary.Round` _output_get))
          (if (!= _display_time _returnvalue)
            (if (>= _display_time 0)
              (bind _output_get_2 (set `self.display time` _returnvalue))
              (if (== (mod _output_get_2 (`self.respawnCooldown`)) 0)
                (`KismetSystemLibrary.PrintString` "SPAWN")
                ;;[1 1 1] Spawning
                (`self.ChooseSpawnZone`)
                (`self.choose Survival wave`)
                (`EnemyPool.UpdateEnemyTargets` (`EnemySpawner.enemyPool` _spawner) (`self.Defense Pod`))
                (`KismetSystemLibrary.PrintString` "POD TARGETED")
                (for _array_element (`MMEnemyWave_DataAsset.spawnList` (`|GetArrayItem` (`MMArenaChallenge_DataAsset.spawnList` (`self.currentArenaChallenge`)) (`self.currentWave`)))
                  (set `EnemySpawner.ActorToSpawn` _array_element _spawner)
                  (`self.K2_SetActorLocation` _spawner (`KismetMathLibrary.RandomPointInBoundingBox` (`SceneComponent.K2_GetComponentLocation` _spawnzone) (`BoxComponent.GetScaledBoxExtent` _spawnzone)) false true)
                  (`EnemySpawner.SpawnEnemy` _spawner)
                  (set `self.EnemyCount` (+ (`self.EnemyCount`) 1)))))))))))

(fn `UserConstructionScript`
  (`parent.UserConstructionScript`))