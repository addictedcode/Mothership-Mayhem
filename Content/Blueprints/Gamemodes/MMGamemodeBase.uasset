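; Base gamemode that stocks the mod shop with randomly generated weapon mods at BeginPlay.
; GenerateNewMods picks random MMModDataAssets through the Asset Registry and stores scaled copies in MMGameInstance's GeneratedModShopMods.
; ScaleMod instantiates each mod, multiplying additive stats by the player's FameRank and copying multiplicative stats unchanged.
; Arena challenge events and SpawnWave are empty; their spawning and win logic is left disconnected.
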(event `self.ReceiveBeginPlay`
  (`self.GenerateNewModsEvent`))

(event `GenerateNewModsEvent`
  (`self.Generate New Mods`)
  (`KismetSystemLibrary.PrintString` "Mods Generated"))

(event `StartArenaChallenge`)

(event `ClearArenaChallenge`)

(fn `Generate New Mods`
  (for _ (range 4)
    ;[1 1 1] Getting Mod Data Asset
    (bind _outassetdata (`AssetRegistry.GetAssetsByClass` (`AssetRegistryHelpers.GetAssetRegistry`) "MMModDataAsset" false))
    (bind _asmmmod_data_asset (cast `MMModDataAsset` (`AssetRegistryHelpers.GetAsset` (`|GetArrayItem` _outassetdata (`KismetMathLibrary.RandomInteger` (`KismetArrayLibrary.Array_Length` _outassetdata))))))
    ;[1 1 1] Scaling the Mod
    (bind _mod_output (`self.Scale Mod` _asmmmod_data_asset))
    ;[1 1 1] Adding Mod to Game Instance
    (bind _asmmgame_instance (cast `/Game/Blueprints/GameInstance/MMGameInstance` (`GameplayStatics.GetGameInstance`)))
    (`KismetArrayLibrary.Array_Add` (`/Game/Blueprints/GameInstance/MMGameInstance.Generated Mod Shop Mods` _asmmgame_instance) _mod_output)))

(fn `Scale Mod`
  (params (`Mod To Scale` :type "MMModDataAsset Object Reference"))
  (returns (`Mod Output` :type "MMModBase Object Reference"))
  (bind _asmmgame_instance (cast `/Game/Blueprints/GameInstance/MMGameInstance` (`GameplayStatics.GetGameInstance`)))
  (set `self.ScalarParam` (`KismetMathLibrary.Conv_IntToDouble` (`/Game/Blueprints/GameInstance/MMGameInstance.FameRank` _asmmgame_instance)))
  (bind _returnvalue (`MMModFactory.InstantiateMod` `Mod To Scale`))
  (bind _returnvalue_2 (`MMModBase.InitializeMod` _returnvalue (make `ModStats` (* (`MMModDataAsset.add_fireRate` `Mod To Scale`) (`self.ScalarParam`)) (* (`MMModDataAsset.add_reloadTime` `Mod To Scale`) (`self.ScalarParam`)) (* (`MMModDataAsset.add_maxAmmo` `Mod To Scale`) (`self.ScalarParam`)) (* (`MMModDataAsset.add_accuracy` `Mod To Scale`) (`self.ScalarParam`)) (* (`MMModDataAsset.add_numberOfProjectilesToShoot` `Mod To Scale`) (`self.ScalarParam`)) (* (`MMModDataAsset.add_damage` `Mod To Scale`) (`self.ScalarParam`)) (* (`MMModDataAsset.add_projectileSpeed` `Mod To Scale`) (`self.ScalarParam`)) (* (`MMModDataAsset.add_projectileGravityScale` `Mod To Scale`) (`self.ScalarParam`))) (make `ModStats` (`MMModDataAsset.multiply_fireRate` `Mod To Scale`) (`MMModDataAsset.multiply_reloadTime` `Mod To Scale`) (`MMModDataAsset.multiply_maxAmmo` `Mod To Scale`) (`MMModDataAsset.multiply_accuracy` `Mod To Scale`) (`MMModDataAsset.multiply_numberOfProjectilesToShoot` `Mod To Scale`) (`MMModDataAsset.multiply_damage` `Mod To Scale`) (`MMModDataAsset.multiply_projectileSpeed` `Mod To Scale`) (`MMModDataAsset.multiply_projectileGravityScale` `Mod To Scale`)) (`MMModDataAsset.projectileClass` `Mod To Scale`) (`MMModDataAsset.name` `Mod To Scale`)))
  (return _returnvalue_2))

(fn `Spawn Wave`)

(fn `UserConstructionScript`)