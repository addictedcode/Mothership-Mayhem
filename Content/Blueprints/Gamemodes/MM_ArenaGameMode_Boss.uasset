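; Boss arena game mode that spawns the current challenge's enemies at random points in spawn zones and tracks player and boss Struggle Points.
; BeginPlay caches the boss, switches on the Extermination HUD and shows a tutorial popup at low difficulty.
; Hit events spawn colored struggle drops, draining boss points gradually but zeroing the player's.
; Boss points below 50 change its reload time; the nested under-20 tier is unreachable.
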(event `self.ReceiveBeginPlay`
  (bind _spawner (`self.Spawner`))
  (bind _spawnzone (`self.spawnZone`))
  (`parent.ReceiveBeginPlay`)
  ;[1 1 1] Init Struggle Points
  (set `self.PlayerStrugglePoints_Current` (`self.PlayerStrugglePoints_Starting`))
  (set `self.BossStrugglePoints_Current` (`self.BossStrugglePoints_Starting`))
  (`KismetSystemLibrary.Delay` 0.1)
  (set `self.EnemyCount` 0)
  (for _array_element (`MMArenaChallenge_DataAsset.spawnList` (`self.currentArenaChallenge`))
    (`self.ChooseSpawnZone`)
    (for _array_element_2 (`MMEnemyWave_DataAsset.spawnList` _array_element)
      ;[1 1 1] Spawning
      (set `EnemySpawner.ActorToSpawn` _array_element_2 _spawner)
      (`self.K2_SetActorLocation` _spawner (`KismetMathLibrary.RandomPointInBoundingBox` (`SceneComponent.K2_GetComponentLocation` _spawnzone) (`BoxComponent.GetScaledBoxExtent` _spawnzone)) false true)
      (`EnemySpawner.SpawnEnemy` _spawner)
      (set `self.EnemyCount` (+ (`self.EnemyCount`) 1))
      (bind _returnvalue (`GameplayStatics.GetActorOfClass` "/Game/Blueprints/Enemies/BossEnemy.BossEnemy_C"))
      (set `self.boss` _returnvalue)))
  (`KismetSystemLibrary.PrintString` (`KismetStringLibrary.Conv_IntToString` (`self.EnemyCount`)))
  ;[1 1 1] UI
  (`KismetSystemLibrary.Delay` 0.2)
  (bind _asbp_mmcharacter_base (cast `/Game/Blueprints/Characters/BP_MMCharacterBase` (`GameplayStatics.GetPlayerCharacter` 0)))
  (`/Game/Blueprints/UI/ArenaChallengeUI/DefenseHUD.Deactivate Defense HUD UI` (`/Game/Blueprints/Characters/BP_MMCharacterBase.DefenseHUDUIReference` _asbp_mmcharacter_base))
  (`/Game/Blueprints/UI/ArenaChallengeUI/ExterminationHUD.Activate Extermination HUD UI` (`/Game/Blueprints/Characters/BP_MMCharacterBase.ExterminationHUDUIReference` _asbp_mmcharacter_base))
  (`/Game/Blueprints/UI/ArenaChallengeUI/SurvivalHUD.Deactivate Survival HUD UI` (`/Game/Blueprints/Characters/BP_MMCharacterBase.SurvivalHUDUIReference` _asbp_mmcharacter_base))
  (if (<= (`MMArenaChallenge_DataAsset.difficultyLevel` (`self.currentArenaChallenge`)) 2)
    (set `self.isTutorial` true)
    (`KismetSystemLibrary.Delay` 0.2)
    (bind _asbp_mmcharacter_base_2 (cast `/Game/Blueprints/Characters/BP_MMCharacterBase` (`GameplayStatics.GetPlayerCharacter` 0)))
    (`/Game/Blueprints/UI/HUD/HUD.OpenPopUp` (`/Game/Blueprints/Characters/BP_MMCharacterBase.HUDUIReference` _asbp_mmcharacter_base_2) "This is the Boss Game Mode!   \nYour goal is to defeat the large enemy in front of you! \nThe Struggle Meter in the top corners dictate the flow of battle. \nIf you have higher struggle points, you get buffs and deal more damage. If the enemy has higher struggle points, it gets tankier and receives less damage. However, if the enemy has lower struggle points, he starts getting aggressive and goes berserk!")
    (else
      (set `self.isTutorial` false))))

(event `Boss Hit`
  (params (`Boss Location` :type "Vector Structure"))
  (bind _returnvalue (- (`self.BossStrugglePoints_Current`) 1))
  (for _ (range (+ (`KismetMathLibrary.RandomIntegerInRange` 1 5) 1))
    (if (not (< _returnvalue 0))
      (set `self.BossStrugglePoints_Current` _returnvalue)
      (`|SpawnActorFromClass` "/Game/Blueprints/Drops/RedStruggleDrops.RedStruggleDrops_C" (`KismetMathLibrary.Conv_VectorToTransform` `Boss Location`) "AdjustIfPossibleButAlwaysSpawn" "OverrideRootScale" null null)
      (if (< (`self.BossStrugglePoints_Current`) 50)
        (`AICharacter.setTimeToReload` (`self.boss`) 1.5)
        (elif (< (`self.BossStrugglePoints_Current`) 20)
          (`AICharacter.setTimeToReload` (`self.boss`) 1.0))))))

(event `Player Hit`
  (params (`Player Location ` :type "Vector Structure"))
  (for _ (range (+ (`KismetMathLibrary.RandomIntegerInRange` 1 5) 1))
    (if (not (< (- (`self.PlayerStrugglePoints_Current`) 1) 0))
      (set `self.PlayerStrugglePoints_Current` 0)
      (`|SpawnActorFromClass` "/Game/Blueprints/Drops/BlueStruggleDrops.BlueStruggleDrops_C" (`KismetMathLibrary.Conv_VectorToTransform` `Player Location `) "AdjustIfPossibleButAlwaysSpawn" "OverrideRootScale" null null))))

(fn `UserConstructionScript`
  (`parent.UserConstructionScript`))