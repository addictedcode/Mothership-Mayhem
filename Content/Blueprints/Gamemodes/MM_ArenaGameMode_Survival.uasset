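; Survival arena game mode that wins the challenge once no enemies remain and the time has run out.
; Tick drains the morale meter by a fixed per-frame step, not scaled by delta time, and checks the win condition.
; EnemyKilled adds morale, divides the current respawn cooldown by a clamped morale tier, decrements the enemy count and rechecks the win for Survival challenges.
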(event `self.ReceiveTick`
  (params (DeltaSeconds :type "Float (single-precision)"))
  (`parent.ReceiveTick` DeltaSeconds)
  (set `self.MoraleMeter` (- (`self.MoraleMeter`) (* (`self.Morale Decrease Rate`) 0.01 1.0)))
  (if (<= (`self.EnemyCount`) 0)
    (if (<= (`self.time`) 0.0)
      (`self.WinArenaChallenge`))))

(event `self.EnemyKilled`
  ;[1 1 1] Morale
  (bind _output_get (set `self.MoraleMeter` (+ (`self.MoraleMeter`) (* 5.0 (`self.Morale Gain Multiplier`)))))
  (set `self.respawnCooldown` (`KismetMathLibrary.Clamp` (/ (`self.respawnCooldown`) (`KismetMathLibrary.Clamp` (`KismetMathLibrary.FTrunc` (/ _output_get 100.0)) 1 10)) 2 10))
  ;[1 1 1] Enemy Count
  (bind _result (`/Engine/EditorBlueprintResources/StandardMacros.DecrementInt` (`self.EnemyCount`))
    (:`  `
      (bind _output_get_2 (set `self.EnemyCount` _result))
      (if (<= _output_get_2 0)
        (switch `MMChallengeType` (`self.Current Challenge Type`)
          (:`Survival`
            (if (<= (`self.time`) 0.0)
              (`self.WinArenaChallenge`))))
        (else
          (`KismetSystemLibrary.PrintString` (`KismetStringLibrary.Conv_IntToString` _output_get_2)))))))

(fn `UserConstructionScript`
  (`parent.UserConstructionScript`))