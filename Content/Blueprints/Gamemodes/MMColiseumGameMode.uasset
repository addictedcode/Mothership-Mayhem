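; Coliseum game mode that tracks remaining enemies and handles the victory condition.
; Each EnemyDied event decrements EnemyNum.
; At zero, it sets the player HUD end text to a win message, slows global time, and after a short delay loads the PreparationArea level.
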(event `EnemyDied`
  (bind _output_get (set `self.EnemyNum` (- (`self.EnemyNum`) 1)))
  (if (== _output_get 0)
    (bind _asbp_mmcharacter_base (cast `/Game/Blueprints/Characters/BP_MMCharacterBase` (`GameplayStatics.GetPlayerCharacter` 0)))
    (set `/Game/Blueprints/UI/HUD/HUD.EndText` "YOU WIN :)" (`/Game/Blueprints/Characters/BP_MMCharacterBase.HUDUIReference` _asbp_mmcharacter_base))
    (`GameplayStatics.SetGlobalTimeDilation` 0.2)
    (`KismetSystemLibrary.Delay` 0.3)
    (`GameplayStatics.OpenLevel` "PreparationArea")))

(fn `UserConstructionScript`
  (`parent.UserConstructionScript`))