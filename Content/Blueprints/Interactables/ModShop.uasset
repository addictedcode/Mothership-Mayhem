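; Interactable mod shop actor that stocks five randomly generated weapon mods for the player to buy.
; On BeginPlay it registers itself on the player character and rolls placeholder names, random stats, icon and price for each mod; GenerateNewMods rerolls them and GetMods returns them.
; Its box overlap sets or clears the HUD purchase prompt, and interacting activates the character's mod shop UI.
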(event `self.ReceiveBeginPlay`
  (bind _asbp_mmcharacter_base (cast `/Game/Blueprints/Characters/BP_MMCharacterBase` (`GameplayStatics.GetPlayerCharacter` 0)))
  (set `/Game/Blueprints/Characters/BP_MMCharacterBase.ModShopGenReference` self _asbp_mmcharacter_base)
  (`self.GenerateNewMods` :!label _label))

(event `Generate New Mods`
  (goto _label))

(event `self.Interactable.OnInteract`
  (params (Context :type "Object Object Reference"))
  (`KismetSystemLibrary.PrintString` "Generate")
  ;[1 1 1] ActivateModShop
  (bind _asbp_mmcharacter_base (cast `/Game/Blueprints/Characters/BP_MMCharacterBase` (`GameplayStatics.GetPlayerCharacter` 0))
    (:`then`
      (`/Game/Blueprints/UI/ModShop/ModShopUI.ActivateModShop` (`/Game/Blueprints/Characters/BP_MMCharacterBase.ModShopUIReference` _asbp_mmcharacter_base))
      (`KismetSystemLibrary.PrintString` "Yes UI"))
    (:`CastFailed`
      (`KismetSystemLibrary.PrintString` "No UI"))))

(event `self.Box.OnComponentBeginOverlap`
  (params (OverlappedComponent :type "PrimitiveComponent Object Reference") (OtherActor :type "Actor Object Reference") (OtherComp :type "PrimitiveComponent Object Reference") (OtherBodyIndex :type Integer) (bFromSweep :type Boolean) (SweepResult :type "HitResult Structure (by ref)"))
  (bind _asbp_mmcharacter_base (cast `/Game/Blueprints/Characters/BP_MMCharacterBase` (`GameplayStatics.GetPlayerCharacter` 0)))
  (set `/Game/Blueprints/UI/HUD/HUD.Interactable Text` "Press E to buy Mods" (`/Game/Blueprints/Characters/BP_MMCharacterBase.HUDUIReference` _asbp_mmcharacter_base)))

(event `self.Box.OnComponentEndOverlap`
  (params (OverlappedComponent :type "PrimitiveComponent Object Reference") (OtherActor :type "Actor Object Reference") (OtherComp :type "PrimitiveComponent Object Reference") (OtherBodyIndex :type Integer))
  (bind _asbp_mmcharacter_base (cast `/Game/Blueprints/Characters/BP_MMCharacterBase` (`GameplayStatics.GetPlayerCharacter` 0)))
  (set `/Game/Blueprints/UI/HUD/HUD.Interactable Text` "" (`/Game/Blueprints/Characters/BP_MMCharacterBase.HUDUIReference` _asbp_mmcharacter_base)))

(fn `GenerateMod`
  (returns (Mod :type "/Game/Blueprints/UI/ModShop/TempMod Structure"))
  (return (make `/Game/Blueprints/UI/ModShop/TempMod` (`KismetTextLibrary.Conv_StringToText` (`KismetStringLibrary.Concat_StrStr` "ModName_" (`KismetStringLibrary.Conv_IntToString` (`KismetMathLibrary.RandomIntegerInRange` 0 10)))) (`KismetTextLibrary.Conv_StringToText` (`KismetStringLibrary.Concat_StrStr` "ModDescription_" (`KismetStringLibrary.Conv_IntToString` (`KismetMathLibrary.RandomIntegerInRange` 0 10)))) (`KismetMathLibrary.RandomIntegerInRange` 0 10) (`KismetMathLibrary.RandomFloatInRange` 0.9 1.1) (`KismetMathLibrary.RandomFloatInRange` 0.9 1.1) (`KismetMathLibrary.RandomIntegerInRange` 0 10) (`KismetMathLibrary.RandomFloatInRange` 1.0 1.0) (`|GetArrayItem` (`self.Images`) (`KismetMathLibrary.RandomIntegerInRange` 0 9)) (`KismetMathLibrary.RandomIntegerInRange` 1 10))))

(fn `GenerateNewMods`
  (bind _mod (`self.GenerateMod`))
  (bind _mod_2 (`self.GenerateMod`))
  (bind _mod_3 (`self.GenerateMod`))
  (bind _mod_4 (`self.GenerateMod`))
  (bind _mod_5 (`self.GenerateMod`))
  (set `self.Mod_0` _mod)
  (set `self.Mod_1` _mod_2)
  (set `self.Mod_2` _mod_3)
  (set `self.Mod_3` _mod_4)
  (set `self.Mod_4` _mod_5))

(fn `GetMods`
  (returns (Mods :type "Array of /Game/Blueprints/UI/ModShop/TempMod Structure"))
  (return (`|MakeArray` (`self.Mod_0`) (`self.Mod_1`) (`self.Mod_2`) (`self.Mod_3`) (`self.Mod_4`))))

(fn `UserConstructionScript`)