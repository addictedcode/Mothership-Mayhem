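; Target dummy that shows floating damage numbers when struck by projectiles, without tracking health or applying damage.
; Capsule hit and begin-overlap events each filter for MMProjectileBase and spawn a DamagePopUP widget with the projectile's rounded damage.
; The hit location or sweep impact point is projected to screen space for the first player to place the popup.
; The hit event also prints a debug string on every contact.
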(event `self.Capsule.OnComponentHit`
  (params (HitComponent :type "PrimitiveComponent Object Reference") (OtherActor :type "Actor Object Reference") (OtherComp :type "PrimitiveComponent Object Reference") (NormalImpulse :type "Vector Structure") (Hit :type "HitResult Structure (by ref)"))
  (`KismetSystemLibrary.PrintString` "Hello")
  ;[1 1 1] On Hit
  (bind _asmmprojectile_base (cast `MMProjectileBase` OtherActor))
  (if true
    (bind _returnvalue (`|CreateWidget` "/Game/Blueprints/UI/ArenaChallengeUI/DamagePopUP.DamagePopUP_C"))
    (`UserWidget.AddToViewport` _returnvalue 0)
    (`/Game/Blueprints/UI/ArenaChallengeUI/DamagePopUP.Damage Text Pop Up Event` _returnvalue (`KismetMathLibrary.Round` (`MMProjectileBase.damage` _asmmprojectile_base)) (`GameplayStatics.ProjectWorldToScreen` (`GameplayStatics.GetPlayerController` 0) (`.Location` (`GameplayStatics.BreakHitResult` Hit)) true))))

(event `self.Capsule.OnComponentBeginOverlap`
  (params (OverlappedComponent :type "PrimitiveComponent Object Reference") (OtherActor :type "Actor Object Reference") (OtherComp :type "PrimitiveComponent Object Reference") (OtherBodyIndex :type Integer) (bFromSweep :type Boolean) (SweepResult :type "HitResult Structure (by ref)"))
  ;[1 1 1] On Collision
  (bind _asmmprojectile_base (cast `MMProjectileBase` OtherActor))
  (if true
    (bind _returnvalue (`|CreateWidget` "/Game/Blueprints/UI/ArenaChallengeUI/DamagePopUP.DamagePopUP_C"))
    (`UserWidget.AddToViewport` _returnvalue 0)
    (`/Game/Blueprints/UI/ArenaChallengeUI/DamagePopUP.Damage Text Pop Up Event` _returnvalue (`KismetMathLibrary.Round` (`MMProjectileBase.damage` _asmmprojectile_base)) (`GameplayStatics.ProjectWorldToScreen` (`GameplayStatics.GetPlayerController` 0) (`.ImpactPoint` (`GameplayStatics.BreakHitResult` SweepResult)) true))))

(fn `UserConstructionScript`)