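; Cheering crowd actor for the Survival arena that bobs its Billboard along a sine wave driven by the game mode's MoraleMeter.
; A random starting phase desynchronizes instances, and each Tick advances it faster as morale rises, with morale also scaling the step size.
; The offset compounds on the current relative transform each frame, making motion frame-rate dependent, and the vector-to-transform conversion resets rotation and scale.
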(event `self.ReceiveBeginPlay`
  (set `self.NewVar_0` (`KismetMathLibrary.RandomFloatInRange` 0.0 100.0)))

(event `self.ReceiveTick`
  (params (DeltaSeconds :type "Float (single-precision)"))
  (bind _billboard (`self.Billboard`))
  (bind _asmm_arena_game_mode_survival (cast `/Game/Blueprints/Gamemodes/MM_ArenaGameMode_Survival` (`GameplayStatics.GetGameMode`)))
  (bind _moralemeter (`/Game/Blueprints/Gamemodes/MM_ArenaGameMode_Survival.MoraleMeter` _asmm_arena_game_mode_survival))
  (bind _output_get (set `self.NewVar_0` (+ (`self.NewVar_0`) (* DeltaSeconds _moralemeter 2.0))))
  (`SceneComponent.K2_SetRelativeTransform` _billboard (`KismetMathLibrary.Conv_VectorToTransform` (`KismetMathLibrary.TransformLocation` (`SceneComponent.GetRelativeTransform` _billboard) (`KismetMathLibrary.MakeVector` 0.0 0.0 (* (`KismetMathLibrary.DegSin` _output_get) 3.0 (/ _moralemeter 100.0))))) false false))

(fn `UserConstructionScript`)