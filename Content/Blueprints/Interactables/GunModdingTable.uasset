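; GunModdingTable is an interactable world actor that lets the player open the gun modding table to customize weapons.
; On interact, it casts the player character to BP_MMCharacterBase and activates its MMGunModdingTableReference.
; A box trigger sets and clears the HUD prompt text on overlap begin and end, without checking which actor overlapped.
; An unconnected call to the older GunModdingTableReference remains.
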(event `self.Interactable.OnInteract`
  (params (Context :type "Object Object Reference"))
  ;[1 1 1] Activate Gun Modding Table
  (bind _asbp_mmcharacter_base (cast `/Game/Blueprints/Characters/BP_MMCharacterBase` (`GameplayStatics.GetPlayerCharacter` 0)))
  (`/Game/Blueprints/UI/GunModdingTable/MM_GunModdingTable_UI.Activate MM Gun Modding Table` (`/Game/Blueprints/Characters/BP_MMCharacterBase.MM_GunModdingTableReference` _asbp_mmcharacter_base)))

(event `self.Box.OnComponentBeginOverlap`
  (params (OverlappedComponent :type "PrimitiveComponent Object Reference") (OtherActor :type "Actor Object Reference") (OtherComp :type "PrimitiveComponent Object Reference") (OtherBodyIndex :type Integer) (bFromSweep :type Boolean) (SweepResult :type "HitResult Structure (by ref)"))
  (bind _asbp_mmcharacter_base (cast `/Game/Blueprints/Characters/BP_MMCharacterBase` (`GameplayStatics.GetPlayerCharacter` 0)))
  (set `/Game/Blueprints/UI/HUD/HUD.Interactable Text` "Press E to customize Guns" (`/Game/Blueprints/Characters/BP_MMCharacterBase.HUDUIReference` _asbp_mmcharacter_base)))

(event `self.Box.OnComponentEndOverlap`
  (params (OverlappedComponent :type "PrimitiveComponent Object Reference") (OtherActor :type "Actor Object Reference") (OtherComp :type "PrimitiveComponent Object Reference") (OtherBodyIndex :type Integer))
  (bind _asbp_mmcharacter_base (cast `/Game/Blueprints/Characters/BP_MMCharacterBase` (`GameplayStatics.GetPlayerCharacter` 0)))
  (set `/Game/Blueprints/UI/HUD/HUD.Interactable Text` "" (`/Game/Blueprints/Characters/BP_MMCharacterBase.HUDUIReference` _asbp_mmcharacter_base)))

(fn `UserConstructionScript`)