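; Interactable repair station for the defense arena mode that spends held scraps to heal the DefensePod.
; A box overlap shows or clears a "Press E to repair Scraps Generator" prompt on the character's HUD.
; On interact, it adds the game mode's HeldScraps to the pod's HP, capped at MaxHP.
; All held scraps are then zeroed, so any surplus beyond full health is lost.
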(event `self.Interactable.OnInteract`
  (params (Context :type "Object Object Reference"))
  ;[1 1 1] Activate Gun Modding Table
  (cast `/Game/Blueprints/Characters/BP_MMCharacterBase` (`GameplayStatics.GetPlayerCharacter` 0))
  (bind _asmm_arena_game_mode_defense (cast `/Game/Blueprints/Gamemodes/MM_ArenaGameMode_Defense` (`GameplayStatics.GetGameMode`)))
  (bind _defense_pod (`/Game/Blueprints/Gamemodes/MM_ArenaGameMode.Defense Pod` _asmm_arena_game_mode_defense))
  (bind _returnvalue (+ (`/Game/Blueprints/Interactables/DefensePod.HP` _defense_pod) (`/Game/Blueprints/Gamemodes/MM_ArenaGameMode_Defense.HeldScraps` _asmm_arena_game_mode_defense)))
  (bind _max_hp (`/Game/Blueprints/Interactables/DefensePod.Max HP` _defense_pod))
  (if (>= _returnvalue _max_hp)
    (set `/Game/Blueprints/Interactables/DefensePod.HP` _max_hp _defense_pod)
    (else
      (set `/Game/Blueprints/Interactables/DefensePod.HP` _returnvalue _defense_pod)))
  (set `/Game/Blueprints/Gamemodes/MM_ArenaGameMode_Defense.HeldScraps` 0 _asmm_arena_game_mode_defense))

(event `self.Box.OnComponentBeginOverlap`
  (params (OverlappedComponent :type "PrimitiveComponent Object Reference") (OtherActor :type "Actor Object Reference") (OtherComp :type "PrimitiveComponent Object Reference") (OtherBodyIndex :type Integer) (bFromSweep :type Boolean) (SweepResult :type "HitResult Structure (by ref)"))
  (bind _asbp_mmcharacter_base (cast `/Game/Blueprints/Characters/BP_MMCharacterBase` OtherActor))
  (set `/Game/Blueprints/UI/HUD/HUD.Interactable Text` "Press E to repair Scraps Generator" (`/Game/Blueprints/Characters/BP_MMCharacterBase.HUDUIReference` _asbp_mmcharacter_base)))

(event `self.Box.OnComponentEndOverlap`
  (params (OverlappedComponent :type "PrimitiveComponent Object Reference") (OtherActor :type "Actor Object Reference") (OtherComp :type "PrimitiveComponent Object Reference") (OtherBodyIndex :type Integer))
  (bind _asbp_mmcharacter_base (cast `/Game/Blueprints/Characters/BP_MMCharacterBase` OtherActor))
  (set `/Game/Blueprints/UI/HUD/HUD.Interactable Text` "" (`/Game/Blueprints/Characters/BP_MMCharacterBase.HUDUIReference` _asbp_mmcharacter_base)))

(fn `UserConstructionScript`)