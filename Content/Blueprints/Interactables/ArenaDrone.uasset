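; Arena drone actor that hovers in place with a bobbing motion while turning to face the first player's pawn.
; Each tick sets the static mesh's relative Z from a sine of the actor's lifetime, replacing any authored height offset.
; The mesh's world rotation follows a look-at toward the player, with pitch inverted and yaw offset, apparently to match the model's orientation.
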(event `self.ReceiveTick`
  (params (DeltaSeconds :type "Float (single-precision)"))
  (bind _staticmesh (`self.StaticMesh`))
  (bind _staticmesh_2 (`self.StaticMesh`))
  (`SceneComponent.K2_SetRelativeLocation` _staticmesh_2 (`KismetMathLibrary.MakeVector` (.x (`SceneComponent.RelativeLocation` _staticmesh_2)) (.y (`SceneComponent.RelativeLocation` _staticmesh_2)) (* (`KismetMathLibrary.DegSin` (* (`self.GetGameTimeSinceCreation`) 100.0)) 20.0)) false false)
  (`SceneComponent.K2_SetWorldRotation` _staticmesh (`KismetMathLibrary.MakeRotator` (.roll (`KismetMathLibrary.FindLookAtRotation` (`SceneComponent.K2_GetComponentLocation` _staticmesh) (`self.K2_GetActorLocation` (`GameplayStatics.GetPlayerPawn` 0)))) (* (.pitch (`KismetMathLibrary.FindLookAtRotation` (`SceneComponent.K2_GetComponentLocation` _staticmesh) (`self.K2_GetActorLocation` (`GameplayStatics.GetPlayerPawn` 0)))) -1.0) (+ (.yaw (`KismetMathLibrary.FindLookAtRotation` (`SceneComponent.K2_GetComponentLocation` _staticmesh) (`self.K2_GetActorLocation` (`GameplayStatics.GetPlayerPawn` 0)))) 270.0)) false false))

(fn `UserConstructionScript`)