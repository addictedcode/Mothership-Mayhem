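; Spaceship sliding door that opens automatically when a BP_MMCharacterBase character enters its trigger and closes when one leaves.
; BeginPlay caches both panels' default relative transforms, and DoorTrigger overlaps toggle the IsOpen flag.
; Tick continuously VInterpTo's each panel toward a fixed sideways offset or its cached position, teleporting without sweep.
; The open state is a single boolean, so any character exiting closes the door even if others remain inside.
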(event `self.ReceiveTick`
  (params (DeltaSeconds :type "Float (single-precision)"))
  (bind _right_door (`self.Right Door`))
  (bind _left_door (`self.Left Door`))
  (bind _right_door_2 (`self.Right Door`))
  (bind _left_door_2 (`self.Left Door`))
  (if (`self.isOpen`)
    (`SceneComponent.K2_SetRelativeLocation` _left_door_2 (`KismetMathLibrary.VInterpTo` (`SceneComponent.RelativeLocation` _left_door_2) (0.0 -200.0 0.0) DeltaSeconds 5.0) false true)
    (`SceneComponent.K2_SetRelativeLocation` _right_door (`KismetMathLibrary.VInterpTo` (`SceneComponent.RelativeLocation` _right_door) (0.0 200.0 0.0) DeltaSeconds 5.0) false true)
    (else
      (`SceneComponent.K2_SetRelativeLocation` _left_door (`KismetMathLibrary.VInterpTo` (`SceneComponent.RelativeLocation` _left_door) (.location (`self.Left Door Default Position`)) DeltaSeconds 5.0) false true)
      (`SceneComponent.K2_SetRelativeLocation` _right_door_2 (`KismetMathLibrary.VInterpTo` (`SceneComponent.RelativeLocation` _right_door_2) (.location (`self.Right Door Default Position_0`)) DeltaSeconds 5.0) false true))))

(event `self.ReceiveBeginPlay`
  (set `self.Left Door Default Position` (`SceneComponent.GetRelativeTransform` (`self.Left Door`)))
  (set `self.Right Door Default Position_0` (`SceneComponent.GetRelativeTransform` (`self.Right Door`))))

(event `self.Door Trigger.OnComponentBeginOverlap`
  (params (OverlappedComponent :type "PrimitiveComponent Object Reference") (OtherActor :type "Actor Object Reference") (OtherComp :type "PrimitiveComponent Object Reference") (OtherBodyIndex :type Integer) (bFromSweep :type Boolean) (SweepResult :type "HitResult Structure (by ref)"))
  (cast `/Game/Blueprints/Characters/BP_MMCharacterBase` OtherActor)
  (set `self.isOpen` true))

(event `self.Door Trigger.OnComponentEndOverlap`
  (params (OverlappedComponent :type "PrimitiveComponent Object Reference") (OtherActor :type "Actor Object Reference") (OtherComp :type "PrimitiveComponent Object Reference") (OtherBodyIndex :type Integer))
  (cast `/Game/Blueprints/Characters/BP_MMCharacterBase` OtherActor)
  (set `self.isOpen` false))

(fn `UserConstructionScript`)