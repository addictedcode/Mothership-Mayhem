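; Battery drop pickup for the Defense arena mode that adds a small random amount to the game mode's HeldScraps.
; On spawn it launches its mesh with a random force, then spins every tick and eases toward PlayerTarget when valid.
; Actor overlap sets that target, though its Player tag check tests the drop itself rather than the overlapping actor.
; Mesh overlap with a Player-tagged actor grants the scraps and destroys the drop.
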(event `self.ReceiveBeginPlay`
  (`PrimitiveComponent.AddForce` (`self.StaticMesh`) (`KismetMathLibrary.MakeVector` (`KismetMathLibrary.RandomFloatInRange` 5000.0 10000.0) (`KismetMathLibrary.RandomFloatInRange` 5000.0 10000.0) (`KismetMathLibrary.RandomFloatInRange` 10000.0 15000.0)) "None" true))

(event `self.ReceiveTick`
  (params (DeltaSeconds :type "Float (single-precision)"))
  (bind _playertarget (`self.PlayerTarget`))
  (`self.K2_AddActorWorldRotation` (`KismetMathLibrary.MakeRotator` 0.0 0.0 (* DeltaSeconds 180.0)))
  (if (`KismetSystemLibrary.IsValid` _playertarget)
    (`self.K2_SetActorLocation` (`KismetMathLibrary.VInterpTo` (`self.K2_GetActorLocation` self) (`self.K2_GetActorLocation` _playertarget) DeltaSeconds 1.0) false true)))

(event `self.ReceiveActorBeginOverlap`
  (params (OtherActor :type "Actor Object Reference"))
  (if (`self.ActorHasTag` "Player")
    (set `self.PlayerTarget` OtherActor)))

(event `self.StaticMesh.OnComponentBeginOverlap`
  (params (OverlappedComponent :type "PrimitiveComponent Object Reference") (OtherActor :type "Actor Object Reference") (OtherComp :type "PrimitiveComponent Object Reference") (OtherBodyIndex :type Integer) (bFromSweep :type Boolean) (SweepResult :type "HitResult Structure (by ref)"))
  (if (`self.ActorHasTag` OtherActor "Player")
    (bind _asmm_arena_game_mode_defense (cast `/Game/Blueprints/Gamemodes/MM_ArenaGameMode_Defense` (`GameplayStatics.GetGameMode`)))
    (set `/Game/Blueprints/Gamemodes/MM_ArenaGameMode_Defense.HeldScraps` (+ (`/Game/Blueprints/Gamemodes/MM_ArenaGameMode_Defense.HeldScraps` _asmm_arena_game_mode_defense) (`KismetMathLibrary.RandomIntegerInRange` 1 5)) _asmm_arena_game_mode_defense)
    (`self.K2_DestroyActor`)))

(fn `UserConstructionScript`)