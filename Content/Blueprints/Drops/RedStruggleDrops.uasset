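; RedStruggleDrops is a pickup that awards a struggle point to whoever touches it, player or boss, in the boss arena.
; On BeginPlay it launches its Sphere with a randomized, upward-biased force.
; An overlap on PlayerDetector by a player character or BossEnemy increments that side's current struggle points on MM_ArenaGameMode_Boss and destroys the drop.
; The player branch also prints a debug string.
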(event `self.ReceiveBeginPlay`
  (`PrimitiveComponent.AddForce` (`self.Sphere`) (`KismetMathLibrary.MakeVector` (`KismetMathLibrary.RandomFloatInRange` -2000.0 10000.0) (`KismetMathLibrary.RandomFloatInRange` -2000.0 2000.0) (`KismetMathLibrary.RandomFloatInRange` 10000.0 15000.0)) "None" false))

(event `self.PlayerDetector.OnComponentBeginOverlap`
  (params (OverlappedComponent :type "PrimitiveComponent Object Reference") (OtherActor :type "Actor Object Reference") (OtherComp :type "PrimitiveComponent Object Reference") (OtherBodyIndex :type Integer) (bFromSweep :type Boolean) (SweepResult :type "HitResult Structure (by ref)"))
  (bind _asmm_arena_game_mode_boss (cast `/Game/Blueprints/Gamemodes/MM_ArenaGameMode_Boss` (`GameplayStatics.GetGameMode`)))
  (cast `/Game/Blueprints/Characters/BP_MMCharacterBase` OtherActor
    (:`then`
      (set `/Game/Blueprints/Gamemodes/MM_ArenaGameMode_Boss.PlayerStrugglePoints_Current` (+ (`/Game/Blueprints/Gamemodes/MM_ArenaGameMode_Boss.PlayerStrugglePoints_Current` _asmm_arena_game_mode_boss) 1) _asmm_arena_game_mode_boss)
      (`KismetSystemLibrary.PrintString` "Hello")
      (`self.K2_DestroyActor`))
    (:`CastFailed`
      (cast `/Game/Blueprints/Enemies/BossEnemy` OtherActor)
      (set `/Game/Blueprints/Gamemodes/MM_ArenaGameMode_Boss.BossStrugglePoints_Current` (+ (`/Game/Blueprints/Gamemodes/MM_ArenaGameMode_Boss.BossStrugglePoints_Current` _asmm_arena_game_mode_boss) 1) _asmm_arena_game_mode_boss)
      (`self.K2_DestroyActor`))))

(fn `UserConstructionScript`)