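; MoneyDrop is a money pickup that spins and drifts toward the player, adding a fixed amount to the player's money when collected.
; Actor overlap events set or clear the player target by the "Player" tag.
; Tick rotates the drop and eases it toward that target with VInterpTo, teleporting without sweep.
; The Cube's overlap with the player credits Money on MMGameInstance and destroys the actor.
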(event `self.ReceiveTick`
  (params (DeltaSeconds :type "Float (single-precision)"))
  (bind _playertarget (`self.PlayerTarget`))
  (`self.K2_AddActorWorldRotation` (`KismetMathLibrary.MakeRotator` 0.0 0.0 (* DeltaSeconds 180.0)))
  (if (`KismetSystemLibrary.IsValid` _playertarget)
    (`self.K2_SetActorLocation` (`KismetMathLibrary.VInterpTo` (`self.K2_GetActorLocation` self) (`self.K2_GetActorLocation` _playertarget) DeltaSeconds 1.0) false true)))

(event `self.ReceiveActorBeginOverlap`
  (params (OtherActor :type "Actor Object Reference"))
  (if (`self.ActorHasTag` OtherActor "Player")
    (set `self.PlayerTarget` OtherActor)))

(event `self.ReceiveActorEndOverlap`
  (params (OtherActor :type "Actor Object Reference"))
  (if (`self.ActorHasTag` OtherActor "Player")
    (set `self.PlayerTarget` null)))

(event `self.Cube.OnComponentBeginOverlap`
  (params (OverlappedComponent :type "PrimitiveComponent Object Reference") (OtherActor :type "Actor Object Reference") (OtherComp :type "PrimitiveComponent Object Reference") (OtherBodyIndex :type Integer) (bFromSweep :type Boolean) (SweepResult :type "HitResult Structure (by ref)"))
  (if (`self.ActorHasTag` OtherActor "Player")
    (bind _asmmgame_instance (cast `/Game/Blueprints/GameInstance/MMGameInstance` (`GameplayStatics.GetGameInstance`)))
    (set `/Game/Blueprints/GameInstance/MMGameInstance.Money` (+ (`/Game/Blueprints/GameInstance/MMGameInstance.Money` _asmmgame_instance) 5) _asmmgame_instance)
    (`self.K2_DestroyActor`)))

(fn `UserConstructionScript`)